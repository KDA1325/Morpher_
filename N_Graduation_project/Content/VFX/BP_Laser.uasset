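; BP_Laser is a laser hazard actor that plays a spin sound and tints its Niagara effects orange-red on BeginPlay.
; Each Tick it line-traces from the Sphere on the Camera channel and sets the beam's LaserEnd to the hit or trace end.
; Damage is independent of the trace, applied to the player character when it begins overlapping the Box.
; Impact effect visibility and positioning logic is disconnected and never runs.
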(event OnComponentBeginOverlap(Box)
  (params (OverlappedComponent :type Primitive%20Component%20Object%20Reference) (OtherActor :type Actor%20Object%20Reference) (OtherComp :type Primitive%20Component%20Object%20Reference) (OtherBodyIndex :type Integer) (bFromSweep :type Boolean) (SweepResult :type Hit%20Result%20Structure%20%28by%20ref%29))
  (bind _returnvalue (Game|GetPlayerCharacter 0))
  (if (== OtherActor _returnvalue)
    (Game|Damage|ApplyDamage _returnvalue 3e+01 0 0)))

(event EventBeginPlay
  (Audio|SpawnSoundatLocation "/Game/Sounds/Battle/LazerSpin.LazerSpin" (Transformation|GetActorLocation) "0, 0, 0" 1.0 1.0 0.0 0 0)
  (Effects|Components|ParticleSystem|SetColorParameter (Variables|Default|GetNiagara_Laser) "Color" "(R=1.000000,G=0.075481,B=0.000000,A=1.000000)"))

(event EventTick
  (params (DeltaSeconds :type Float%20%28single-precision%29))
  (bind _sphere (Variables|Default|GetSphere))
  (bind _distance (Variables|Default|GetDistance))
  (bind _returnvalue (Transformation|GetWorldRotation _sphere))
  (bind _returnvalue_2 (Transformation|GetWorldLocation _sphere))
  (bind _returnvalue_3 (* _returnvalue _distance))
  (bind _returnvalue_4 (+ _returnvalue_2 _returnvalue_3))
  (Variables|Default|SetTrace%20End _returnvalue_4) ; 레이저 끝을 저장
  (bind _outhit (Collision|LineTraceByChannel _returnvalue_2 _returnvalue_4 "TraceTypeQuery2" false 0 "None"))
  (Variables|Default|SetbHit (.bblockinghit _outhit))
  (Variables|Default|SetHit%20Location (.location _outhit))
  (Effects|Components|ParticleSystem|SetVectorParameter (Variables|Default|GetNiagara_Laser) "LaserEnd" (select (Variables|Default|GetbHit) (Variables|Default|GetHit%20Location) (Variables|Default|GetTrace%20End))) ; Hit상태, 레이저 끝길이 업뎃
)

(fn ConstructionScript)