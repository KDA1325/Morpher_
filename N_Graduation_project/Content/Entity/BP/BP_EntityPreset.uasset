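; BP_EntityPreset is an entity actor with a preset widget component that faces the player's camera.
; On BeginPlay the widget is hidden.
; Each Tick, once IsSpawned is true, it shows the widget and rotates it with a look-at rotation toward the player camera manager's location, so only its front is seen.
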(event EventBeginPlay
  (Rendering|SetVisibility (Variables|Default|GetEntityPresetWidget) false false))

(event EventTick
  (params (DeltaSeconds :type Float%20%28single-precision%29))
  ;[1 1 1] 위젯이 정면의 모습만 보이도록
  (if (Variables|Default|GetisSpawned)
    (Rendering|SetVisibility (Variables|Default|GetEntityPresetWidget) true false)
    (Transformation|SetWorldRotation (Variables|Default|GetEntityPresetWidget) (Math|Rotator|FindLookatRotation (Transformation|GetActorLocation) (Transformation|GetActorLocation (Game|GetPlayerCameraManager 0))) false false)))

(fn ConstructionScript)