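; Demo-style projectile Blueprint in a stylized magic VFX pack that repeatedly fires a Niagara effect from Start to Target.
; On BeginPlay it spawns the NSProjectile system, and the Travel timeline, with play rate set by Speed, lerps it between the two points without sweeping.
; On arrival it sets the system's Hit parameter, deactivates it, then respawns and relaunches after a short delay.
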(event EventBeginPlay
  (bind _start (Variables|Default|GetStart))
  (bind _returnvalue (Transformation|GetWorldLocation _start))
  (Components|Timeline|SetPlayRate (Variables|Default|GetTravel) (Variables|Components|GetSpeed) :!label _label)
  (bind _returnvalue_2 (Niagara|SpawnSystematLocation (AssetData|GetAsset (Variables|Default|GetNS_Projectile)) _returnvalue))
  (bind _newtrack_0 (Timeline|Travel PlayFromStart)
    (:Update
      (Transformation|SetWorldLocation _returnvalue_2 (Math|Vector|Lerp(Vector) _returnvalue (Transformation|GetWorldLocation (Variables|Default|GetTarget)) _newtrack_0) false false))
    (:Finished
      (Class|NiagaraComponent|SetVariableBool _returnvalue_2 "Hit" true)
      (Components|Activation|Deactivate _returnvalue_2)
      (Utilities|FlowControl|Delay 2.3)
      (goto _label))))

(fn ConstructionScript)