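; BP_ProjectileHit is a VFX preview actor that plays a Niagara projectile and hit effect when NumPad 0 is pressed.
; The key press spawns the projectile system at the Start component and plays the Travel timeline at the Speed play rate.
; The timeline lerps the system toward the Target component.
; On finish, it deactivates the projectile and spawns the hit system at Target, with no collision or gameplay logic.
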(event Input|KeyboardEvents|NumPadZero
  (params (Key :type Key%20Structure))
  (bind _start (Variables|Default|GetStart))
  (bind _target (Variables|Default|GetTarget))
  (bind _returnvalue (Transformation|GetWorldLocation _start))
  (bind _returnvalue_2 (Transformation|GetWorldLocation _target))
  (:Pressed
    (Components|Timeline|SetPlayRate (Variables|Default|GetTravel) (Variables|Components|GetSpeed))
    (bind _returnvalue_3 (Niagara|SpawnSystematLocation (AssetData|GetAsset (Variables|Default|GetNS_Projectile)) _returnvalue))
    (bind _newtrack_0 (Timeline|Travel PlayFromStart)
      (:Update
        (Transformation|SetWorldLocation _returnvalue_3 (Math|Vector|Lerp(Vector) _returnvalue _returnvalue_2 _newtrack_0) false false))
      (:Finished
        (Components|Activation|Deactivate _returnvalue_3)
        (Niagara|SpawnSystematLocation (AssetData|GetAsset (Variables|Default|GetNS_Hit)) _returnvalue_2)))))

(fn ConstructionScript)