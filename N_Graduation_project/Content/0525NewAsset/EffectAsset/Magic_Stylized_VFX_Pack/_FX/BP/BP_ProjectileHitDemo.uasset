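; Demo actor from a VFX pack that shows five elemental Niagara projectiles (Floral, Ice, Magic, Electric, Fire) flying and hitting.
; On BeginPlay, each lane spawns its projectile, and a Speed-scaled timeline lerps it from Start to Target.
; On arrival it deactivates, some first setting a "Hit" variable, and a hit effect spawns.
; Only the Floral lane loops back after a delay, restarting all five lanes together.
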(event EventBeginPlay
  (bind _ns_projectile (Variables|Default|GetNS_Projectile))
  (bind _ns_projectile5 (Variables|Default|GetNS_Projectile5))
  (bind _start5 (Variables|Default|GetStart5))
  (bind _target5 (Variables|Default|GetTarget5))
  (bind _ns_projectile3 (Variables|Default|GetNS_Projectile3))
  (bind _start3 (Variables|Default|GetStart3))
  (bind _ns_projectile4 (Variables|Default|GetNS_Projectile4))
  (bind _target3 (Variables|Default|GetTarget3))
  (bind _ns_projectile2 (Variables|Default|GetNS_Projectile2))
  (bind _start2 (Variables|Default|GetStart2))
  (bind _target2 (Variables|Default|GetTarget2))
  (bind _start (Variables|Default|GetStart))
  (bind _start4 (Variables|Default|GetStart4))
  (bind _target (Variables|Default|GetTarget))
  (bind _target4 (Variables|Default|GetTarget4))
  (bind _returnvalue (Transformation|GetWorldLocation _start3))
  (bind _returnvalue_2 (Transformation|GetWorldLocation _target))
  (bind _returnvalue_3 (Transformation|GetWorldLocation _start5))
  (bind _returnvalue_4 (Transformation|GetWorldLocation _target5))
  (bind _returnvalue_5 (Transformation|GetWorldLocation _start2))
  (bind _returnvalue_6 (Transformation|GetWorldLocation _target2))
  (bind _returnvalue_7 (Transformation|GetWorldLocation _target3))
  (bind _returnvalue_8 (Transformation|GetWorldLocation _start4))
  (bind _returnvalue_9 (Transformation|GetWorldLocation _target4))
  (bind _returnvalue_10 (Transformation|GetWorldLocation _start))
  (Utilities|FlowControl|Sequence :!label _label
    (:then_0
      ;[1 1 1] Floral
      (Components|Timeline|SetPlayRate (Variables|Default|GetTravel) (Variables|Components|GetSpeed))
      (bind _returnvalue_11 (Niagara|SpawnSystematLocation (AssetData|GetAsset _ns_projectile) _returnvalue_10 (Transformation|GetWorldRotation _ns_projectile)))
      (bind _newtrack_0 (Timeline|Travel PlayFromStart)
        (:Update
          (Transformation|SetWorldLocation _returnvalue_11 (Math|Vector|Lerp(Vector) _returnvalue_10 _returnvalue_2 _newtrack_0) false false))
        (:Finished
          (Class|NiagaraComponent|SetVariableBool _returnvalue_11 "Hit" true)
          (Components|Activation|Deactivate _returnvalue_11)
          (Niagara|SpawnSystematLocation (AssetData|GetAsset (Variables|Default|GetNS_Hit)) _returnvalue_2)
          (Utilities|FlowControl|Delay 2.0)
          (goto _label))))
    (:then_1
      ;[1 1 1] Ice
      (Components|Timeline|SetPlayRate (Variables|Default|GetTravel2) (Variables|Components|GetSpeed))
      (bind _returnvalue_12 (Niagara|SpawnSystematLocation (AssetData|GetAsset _ns_projectile2) _returnvalue_5 (Transformation|GetWorldRotation _ns_projectile2)))
      (bind _newtrack_0_2 (Timeline|Travel2 PlayFromStart)
        (:Update
          (Transformation|SetWorldLocation _returnvalue_12 (Math|Vector|Lerp(Vector) _returnvalue_5 _returnvalue_6 _newtrack_0_2) false false))
        (:Finished
          (Components|Activation|Deactivate _returnvalue_12)
          (Niagara|SpawnSystematLocation (AssetData|GetAsset (Variables|Default|GetNS_Hit2)) _returnvalue_6))))
    (:then_2
      ;[1 1 1] Magic
      (Components|Timeline|SetPlayRate (Variables|Default|GetTravel3) (Variables|Components|GetSpeed))
      (bind _returnvalue_13 (Niagara|SpawnSystematLocation (AssetData|GetAsset _ns_projectile3) _returnvalue (Transformation|GetWorldRotation _ns_projectile3)))
      (bind _newtrack_0_3 (Timeline|Travel3 PlayFromStart)
        (:Update
          (Transformation|SetWorldLocation _returnvalue_13 (Math|Vector|Lerp(Vector) _returnvalue _returnvalue_7 _newtrack_0_3) false false))
        (:Finished
          (Class|NiagaraComponent|SetVariableBool _returnvalue_13 "Hit" true)
          (Components|Activation|Deactivate _returnvalue_13)
          (Niagara|SpawnSystematLocation (AssetData|GetAsset (Variables|Default|GetNS_Hit3)) _returnvalue_7))))
    (:then_3
      ;[1 1 1] Electric
      (Components|Timeline|SetPlayRate (Variables|Default|GetTravel4) (Variables|Components|GetSpeed))
      (bind _returnvalue_14 (Niagara|SpawnSystematLocation (AssetData|GetAsset _ns_projectile4) _returnvalue_8 (Transformation|GetWorldRotation _ns_projectile4)))
      (bind _newtrack_0_4 (Timeline|Travel4 PlayFromStart)
        (:Update
          (Transformation|SetWorldLocation _returnvalue_14 (Math|Vector|Lerp(Vector) _returnvalue_8 _returnvalue_9 _newtrack_0_4) false false))
        (:Finished
          (Components|Activation|Deactivate _returnvalue_14)
          (Niagara|SpawnSystematLocation (AssetData|GetAsset (Variables|Default|GetNS_Hit4)) _returnvalue_9))))
    (:then_4
      ;[1 1 1] Fire
      (Components|Timeline|SetPlayRate (Variables|Default|GetTravel%205) (Variables|Components|GetSpeed))
      (bind _returnvalue_15 (Niagara|SpawnSystematLocation (AssetData|GetAsset _ns_projectile5) _returnvalue_3 (Transformation|GetWorldRotation _ns_projectile5)))
      (bind _newtrack_0_5 (Timeline|Travel%205 PlayFromStart)
        (:Update
          (Transformation|SetWorldLocation _returnvalue_15 (Math|Vector|Lerp(Vector) _returnvalue_3 _returnvalue_4 _newtrack_0_5) false false))
        (:Finished
          (Class|NiagaraComponent|SetVariableBool _returnvalue_15 "Hit" true)
          (Components|Activation|Deactivate _returnvalue_15)
          (Niagara|SpawnSystematLocation (AssetData|GetAsset (Variables|Default|GetNS_Hit5)) _returnvalue_4))))))

(fn ConstructionScript)