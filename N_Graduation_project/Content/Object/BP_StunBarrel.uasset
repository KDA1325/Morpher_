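; Stun barrel actor that, once its explosion starts, warns with a color fade and range preview, then explodes and destroys itself.
; BeginPlay sets the delay and radius, sizing the trigger sphere and preview mesh.
; StartExplosion's timeline tints a dynamic material, then after a delay calls EndtExplosion, defined outside this graph, and spawns the explosion particle.
; AnyDamage is empty, and the radial pawn-damage logic is left unconnected.
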(event EventBeginPlay
  ;[1 1 1] 폭발 연출 딜레이 값
  (Variables|Default|SetExplosionDelay 1.0)
  ;[1 1 1] 데미지 반경(반지름)
  (bind _output_get (Variables|Default|SetEffectRadius 200))
  (Components|Sphere|SetSphereRadius (Variables|Default|GetSphere) (Math|Conversions|ToFloat(Integer) _output_get) true)
  (Transformation|SetWorldScale3D (Variables|Default|GetExplosionRangePreview) (Math|Vector|MakeVector (Math|Conversions|ToFloat(Integer) (/ _output_get 25)) (Math|Conversions|ToFloat(Integer) (/ _output_get 25)) 0.1)))

(event EventStartExplosion
  ;[1 1 1] 화약통 점화, 2초 딜레이
  (bind _alpha (Timeline|타임라인 Play)
    (:Update
      (bind _returnvalue (Rendering|Material|CreateDynamicMaterialInstance (Variables|Default|GetBarrel) 0 "/Game/SyntyAsset/PolygonFantasyKingdom_Weapon/Materials/M_PolygonFantasyKingdom_01_A.M_PolygonFantasyKingdom_01_A" "None" :!class /Script/Engine.PrimitiveComponent))
      (Rendering|Material|SetVectorParameterValue _returnvalue "Color" (Math|Color|Lerp(LinearColor) (Variables|Default|GetStartColor) (Variables|Default|GetTargetColor) _alpha) :!class /Script/Engine.MaterialInstanceDynamic)
      (Development|SetHiddeninGame (Variables|Default|GetExplosionRangePreview) false false)
      (Utilities|FlowControl|Delay (Variables|Default|GetExplosionDelay))
      (Class|StunBarrel|EndtExplosion)
      (Effects|SpawnEmitteratLocation "/Game/StarterContent/Particles/P_Explosion.P_Explosion" (Transformation|GetActorLocation) "0, 0, 0" "4.000000,4.000000,4.000000")
      (Actor|DestroyActor))))

(event Game|Damage|EventAnyDamage
  (params (Damage :type Float%20%28single-precision%29) (DamageType :type Damage%20Type%20Object%20Reference) (InstigatedBy :type Controller%20Object%20Reference) (DamageCauser :type Actor%20Object%20Reference))
  ;[1 1 1] 대미지 처리
)

(fn ConstructionScript)