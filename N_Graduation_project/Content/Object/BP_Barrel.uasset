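; BP_Barrel is an explosive barrel that ignites when it takes any damage and blows up after a short delay.
; The ColorFade timeline tints a dynamic material on the mesh and reveals the explosion range preview.
; A Delay chained from the timeline's Update leads to a sphere overlap that damages nearby Pawns.
; The barrel then spawns a scaled-up explosion emitter and destroys itself.
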(event Game|Damage|EventAnyDamage
  (params (Damage :type Float%20%28single-precision%29) (DamageType :type Damage%20Type%20Object%20Reference) (InstigatedBy :type Controller%20Object%20Reference) (DamageCauser :type Actor%20Object%20Reference))
  ;[1 1 1] 대미지 처리
  ;[1 1 1] 화약통 점화, 2초 딜레이
  (bind _alpha (Timeline|ColorFade Play)
    (:Update
      (bind _returnvalue (Rendering|Material|CreateDynamicMaterialInstance (Variables|Default|GetBarrel) 0 "/Game/SyntyAsset/PolygonFantasyKingdom_Weapon/Materials/M_PolygonFantasyKingdom_01_A.M_PolygonFantasyKingdom_01_A" "None" :!class /Script/Engine.PrimitiveComponent))
      (Rendering|Material|SetVectorParameterValue _returnvalue "Color" (Math|Color|Lerp(LinearColor) (Variables|Default|GetStartColor) (Variables|Default|GetTargetColor) _alpha) :!class /Script/Engine.MaterialInstanceDynamic)
      (Development|SetHiddeninGame (Variables|Default|GetExplosionRangePreview) false false)
      (Utilities|FlowControl|Delay 2.0)
      ;[1 1 1] 대미지 범위 측정 및 오브젝트 타입: 폰 탐지
      (bind _outactors (Collision|SphereOverlapActors (Transformation|GetActorLocation) 2e+02 (Utilities|Array|MakeArray "ObjectTypeQuery3") 0))
      ;[1 1 1] 대상 탐색
      (for _array_element _outactors
        (bind _as폰 (Utilities|Casting|CastToPawn _array_element))
        ;[1 1 1] 대미지 발생
        (Game|Damage|ApplyDamage _as폰 5e+01 0 0 "/Script/Engine.DamageType"))
      (Effects|SpawnEmitteratLocation "/Game/StarterContent/Particles/P_Explosion.P_Explosion" (Transformation|GetActorLocation) "0, 0, 0" "4.000000,4.000000,4.000000")
      (Actor|DestroyActor))))

(fn ConstructionScript)