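; BP_RoomTrigger is a one-shot combat room trigger that locks the player in until all spawned entities are gone.
; On the first overlap by BP_ThirdPersonCharacter, it shows the entrance and exit gate walls, spawns an entity from each referenced spawner, then destroys those spawners.
; A looping one-second timer runs CheckEntityCleared, which hides both walls and clears itself once no spawned entity remains valid.
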(event EventBeginPlay
  (Variables|Default|SetbRoomActivated false))

(event Collision|EventActorBeginOverlap
  (params (OtherActor :type Actor%20Object%20Reference))
  (Utilities|Casting|CastToBP_ThirdPersonCharacter OtherActor)
  (if (== (Variables|Default|GetbRoomActivated) false)
    (Variables|Default|SetbRoomActivated true)
    (Utilities|FlowControl|Sequence
      (:then_0
        (Default|ShowGateWall (Variables|Default|GetEntranceWall)))
      (:then_1
        (Default|ShowGateWall (Variables|Default|GetExitWall)))
      (:then_2
        (for _array_element (Variables|Default|GetSpanwers)
          (bind _returnvalue (Class|EntitySpawner|SpawnEntityCharacter _array_element))
          (Utilities|Array|Add (Variables|Default|GetSpanwedEntities) _returnvalue)
          (Actor|DestroyActor _array_element)))
      (:then_3
        (Utilities|Time|SetTimerbyFunctionName 0 "CheckEntityCleared" 1.0 true)))))

(event EventTick
  (params (DeltaSeconds :type Float%20%28single-precision%29)))

(fn ConstructionScript)

(fn CheckEntityCleared
  (Variables|Default|SetAllDead true)
  (for _array_element (Variables|Default|GetSpanwedEntities)
    (Utilities|IsValid _array_element
      (:Is%20Valid
        (Variables|Default|SetAllDead false))))
  (if (Variables|Default|GetAllDead)
    (Utilities|FlowControl|Sequence
      (:then_0
        (Default|HideGateWall (Variables|Default|GetEntranceWall)))
      (:then_1
        (Default|HideGateWall (Variables|Default|GetExitWall)))
      (:then_2
        (Utilities|Time|ClearTimerbyFunctionName 0 "CheckEntityCleared")))))