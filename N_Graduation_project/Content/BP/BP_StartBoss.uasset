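; Boss encounter trigger actor that starts the fight and makes a set of static meshes appear.
; BeginPlay hides the meshes and disables collision on all but one of them.
; Overlapping Box sets BossStart on MyGameInstance and moves the player's follow camera to a high, angled relative view, with no once guard.
; Overlapping Box1 plays an explosion sound and restores visibility and collision, once only.
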(event OnComponentBeginOverlap(Box)
  (params (OverlappedComponent :type Primitive%20Component%20Object%20Reference) (OtherActor :type Actor%20Object%20Reference) (OtherComp :type Primitive%20Component%20Object%20Reference) (OtherBodyIndex :type Integer) (bFromSweep :type Boolean) (SweepResult :type Hit%20Result%20Structure%20%28by%20ref%29))
  (bind _asmy_game_instance (Utilities|Casting|CastToMyGameInstance (Game|GetGameInstance)))
  (Variables|/Script/N_Graduation_project.MyGameInstance|SetBossStart _asmy_game_instance true)
  (bind _asbp_third_person_character (Utilities|Casting|CastToBP_ThirdPersonCharacter (Game|GetPlayerCharacter 0)))
  (Transformation|SetRelativeLocationAndRotation (Variables|/Script/N_Graduation_project.N_Graduation_projectCharacter|GetFollowCamera _asbp_third_person_character) "-300.000000,0.000000,2000.000000" "-70.000000,0.000000,0.000000" false false))

(event OnComponentBeginOverlap(Box1)
  (params (OverlappedComponent :type Primitive%20Component%20Object%20Reference) (OtherActor :type Actor%20Object%20Reference) (OtherComp :type Primitive%20Component%20Object%20Reference) (OtherBodyIndex :type Integer) (bFromSweep :type Boolean) (SweepResult :type Hit%20Result%20Structure%20%28by%20ref%29))
  (if (Variables|Default|Getonce)
    (Audio|PlaySound2D "/Game/StarterContent/Audio/Explosion02.Explosion02" 1.0 1.0 0.0 0 0)
    (Development|SetHiddeninGame (Variables|Default|GetStaticMesh8) false false)
    (Collision|SetCollisionEnabled (Variables|Default|GetStaticMesh9) "QueryAndPhysics")
    (Variables|Default|Setonce false)))

(event EventBeginPlay
  (Development|SetHiddeninGame (Variables|Default|GetStaticMesh8) true false)
  (Collision|SetCollisionEnabled (Variables|Default|GetStaticMesh9) "NoCollision")
  (Variables|Default|Setonce true))

(event Collision|EventActorBeginOverlap
  (params (OtherActor :type Actor%20Object%20Reference)))

(fn ConstructionScript)