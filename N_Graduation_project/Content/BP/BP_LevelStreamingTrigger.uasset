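; Trigger volume that streams connected levels in and out when BP_ThirdPersonCharacter overlaps its box.
; On overlap it records which of AllLevelNames are loaded, writing each to the game instance's SaveRoomName so the last one found remains.
; It then asynchronously loads missing ConnectedLevels and unloads loaded levels outside that list, except the level containing the trigger.
; Several disconnected older and debug node chains never run.
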(event OnComponentBeginOverlap(Box)
  (params (OverlappedComponent :type Primitive%20Component%20Object%20Reference) (OtherActor :type Actor%20Object%20Reference) (OtherComp :type Primitive%20Component%20Object%20Reference) (OtherBodyIndex :type Integer) (bFromSweep :type Boolean) (SweepResult :type Hit%20Result%20Structure%20%28by%20ref%29))
  (bind _currentloadedlevels (Variables|Default|GetCurrentLoadedLevels))
  (Utilities|Casting|CastToBP_ThirdPersonCharacter OtherActor)
  (Utilities|FlowControl|Sequence
    (:then_0
      ;[1 1 1] 오버랩 된 시점에 로드되어있는 레벨 저장
      (Utilities|Set|Clear _currentloadedlevels)
      (bind _result (Utilities|Set|ToArray (Variables|Default|GetAllLevelNames)))
      (for _array_element _result
        (Utilities|IsValid (Class|GameplayStatics|GetStreamingLevel _array_element)
          (:Is%20Valid
            (if (Class|LevelStreaming|IsLevelLoaded (Class|GameplayStatics|GetStreamingLevel _array_element))
              (Utilities|Set|Add _currentloadedlevels _array_element)
              (bind _asmy_game_instance (Utilities|Casting|CastToMyGameInstance (Game|GetGameInstance)))
              (Variables|/Script/N_Graduation_project.MyGameInstance|SetSaveRoomName _asmy_game_instance (Utilities|String|StringToName (Utilities|String|ToString(Name) _array_element))))))))
    (:then_1
      ;[1 1 1] Connected Level 중 로드되어있지 않은 레벨만 로드
      (for _array_element_2 (Variables|Default|GetConnectedLevels)
        (if (not (Utilities|Set|Contains (Variables|Default|GetCurrentLoadedLevels) _array_element_2))
          (Game|LoadStreamLevel(byName) _array_element_2 true))))
    (:then_2
      ;[1 1 1] 로드되어있는 레벨 중 Connected Levels에 없는 레벨 언로드
      (bind _result_2 (Utilities|Set|ToArray (Variables|Default|GetCurrentLoadedLevels)))
      (for _array_element_3 _result_2
        (if (not (Utilities|Array|ContainsItem (Variables|Default|GetConnectedLevels) _array_element_3))
          (if (not (== _array_element_3 (Utilities|GetObjectName (Utilities|GetOuterObject (Class|Actor|GetLevel)))))
            (Game|UnloadStreamLevel(byName) _array_element_3 false)))))))

(fn ConstructionScript)